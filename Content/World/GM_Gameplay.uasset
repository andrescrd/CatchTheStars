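; Gameplay game mode that swaps the on-screen UI and refreshes the star sphere as the game status changes.
; On BeginPlay it caches the actor tagged StarSphereDynamic.
; Each status change maps to a widget class (game HUD or shared level-complete/game-over screen), notifying the previous widget it is hidden before showing the new one.
; Entering Playing also randomizes the star sphere and prints a debug string.
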(event EventBeginPlay
  (bind _outactors (Actor|GetAllActorswithTag "StarSphereDynamic"))
  (bind _asbp_star_sphere_dynamic (Utilities|Casting|CastToBP_StarSphereDynamic (Utilities|Array|Get(acopy) _outactors)))
  (Variables|Default|SetStarSphere _asbp_star_sphere_dynamic))

(event EventOnGameStatusChange
  (params (CurrentGameStatus :type EGameStatusEnum%20Enum :default "Waiting"))
  (bind _returnvalue (Utilities|Select :Index CurrentGameStatus :Waiting 0 :Playing "/Game/UI/WB_Game.WB_Game_C" :Completed "/Game/UI/WB_LevelComplete.WB_LevelComplete_C" :GameOver "/Game/UI/WB_LevelComplete.WB_LevelComplete_C" :Unknown 0))
  (Utilities|FlowControl|Sequence
    (:then_0
      (if (Utilities|IsValidClass _returnvalue)
        (if (Utilities|IsValid (Variables|Default|GetLastWidget))
          (Class|WidgetAnimation|OnHidden(Message) (Variables|Default|GetLastWidget)))
        (bind _returnvalue_2 (UserInterface|CreateWidget _returnvalue))
        (bind _output_get (Variables|Default|SetLastWidget _returnvalue_2))
        (UserInterface|Viewport|AddtoViewport _output_get 0)
        (Class|WidgetAnimation|OnAppear(Message) _output_get)))
    (:then_1
      (if (Utilities|Enum|Equal(Enum) CurrentGameStatus "Playing")
        (Default|RandomStarSphere (Variables|Default|GetStarSphere))
        (Development|PrintString "Hello")))))

(fn ConstructionScript)